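; Debug pawn for comparing stereo capture results: live reference cubes, a static cubemap sphere, a spherical atlas sphere, or the plain scene.
; Left and right SceneCaptureCubes refresh briefly on BeginPlay or U.
; Number keys toggle the view roots, update the stereo atlas and feed its eye textures into dynamic materials created in the construction script.
; Further keys switch stereo and HMD position settings through console commands.
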(event EventBeginPlay
  (bind _leftscenecapturecube (Variables|Default|GetLeftSceneCaptureCube))
  (Class|SceneCaptureComponent|HideActorComponents (Variables|Default|GetRightSceneCaptureCube) self)
  (Utilities|FlowControl|Sequence
    (:then_0
      (Development|PrintString "Updating Reference Captures")
      (Rendering|SetVisibility _leftscenecapturecube true false)
      (Variables|/Script/Engine.SceneCaptureComponent|SetbCaptureEveryFrame _leftscenecapturecube true)
      (Variables|/Script/Engine.SceneCaptureComponent|SetbCaptureEveryFrame (Variables|Default|GetRightSceneCaptureCube) true)
      (Utilities|FlowControl|Delay 0.2)
      (Variables|/Script/Engine.SceneCaptureComponent|SetbCaptureEveryFrame (Variables|Default|GetLeftSceneCaptureCube) false)
      (Variables|/Script/Engine.SceneCaptureComponent|SetbCaptureEveryFrame (Variables|Default|GetRightSceneCaptureCube) false)
      (Rendering|SetVisibility (Variables|Default|GetLeftSceneCaptureCube) false false))
    (:then_1
      (Development|PrintString "Showing Live Scene")
      (Rendering|SetVisibility (Variables|Default|GetRefLiveCube_Root) false true))))

(event Input|KeyboardEvents|5
  (:Pressed
    (Development|PrintString "Showing Live Scene")
    (Rendering|SetVisibility (Variables|Default|GetRefLiveCube_Root) false true)))

(event Input|KeyboardEvents|U
  (bind _leftscenecapturecube (Variables|Default|GetLeftSceneCaptureCube))
  (:Pressed
    (Development|PrintString "Updating Reference Captures")
    (Rendering|SetVisibility _leftscenecapturecube true false)
    (Variables|/Script/Engine.SceneCaptureComponent|SetbCaptureEveryFrame _leftscenecapturecube true)
    (Variables|/Script/Engine.SceneCaptureComponent|SetbCaptureEveryFrame (Variables|Default|GetRightSceneCaptureCube) true)
    (Utilities|FlowControl|Delay 0.2)
    (Variables|/Script/Engine.SceneCaptureComponent|SetbCaptureEveryFrame (Variables|Default|GetLeftSceneCaptureCube) false)
    (Variables|/Script/Engine.SceneCaptureComponent|SetbCaptureEveryFrame (Variables|Default|GetRightSceneCaptureCube) false)
    (Rendering|SetVisibility (Variables|Default|GetLeftSceneCaptureCube) false false)))

(event Input|KeyboardEvents|3
  (:Pressed
    (Rendering|SetVisibility (Variables|Default|GetRefLiveCube_Root) false true)
    (Development|PrintString "Rendering Spherical Atlas")
    (Class|StereoCapturePawn|UpdateStereoAtlas)
    (Rendering|Material|SetTextureParameterValue (Variables|Default|GetM_AtlasSphere_Left) "SphericalTexture" (Variables|Default|GetLeftEyeAtlas))
    (Rendering|Material|SetTextureParameterValue (Variables|Default|GetM_AtlasSphere_Right) "SphericalTexture" (Variables|Default|GetRightEyeAtlas))
    (Development|PrintString "Showing Atlas Sphere ")
    (Rendering|SetVisibility (Variables|Default|GetAtlasSphere_Root) true true)
    (Rendering|SetVisibility (Variables|Default|GetRefLiveCube_Root) false true)))

(event Input|KeyboardEvents|Shift6
  (:Pressed
    (Development|ExecuteConsoleCommand "hmdpos on")
    (Development|ExecuteConsoleCommand "stereo w2m=100")
    (Development|ExecuteConsoleCommand "r.setres 1920x1080")
    (Development|ExecuteConsoleCommand "stereo on")))

(event Input|KeyboardEvents|6
  (:Pressed
    (Development|ExecuteConsoleCommand "hmdpos off")
    (Development|ExecuteConsoleCommand "stereo w2m=0")
    (Development|ExecuteConsoleCommand "r.setres 1920x1080")
    (Development|ExecuteConsoleCommand "stereo on")))

(event Input|KeyboardEvents|1
  (:Pressed
    (Development|PrintString "Showing Live Reference Cubes")
    (Rendering|SetVisibility (Variables|Default|GetRefLiveCube_Root) true true)
    (Rendering|SetVisibility (Variables|Default|GetRefStaticSphere_Root) false true)))

(event Input|KeyboardEvents|2
  (:Pressed
    (Development|PrintString "Showing Static Sphere From Cubemaps")
    (Rendering|SetVisibility (Variables|Default|GetRefStaticSphere_Root) true true)
    (Rendering|SetVisibility (Variables|Default|GetRefLiveCube_Root) false true)))

(event Input|KeyboardEvents|4
  (:Pressed
    (Rendering|Material|SetTextureParameterValue (Variables|Default|GetM_AtlasSphere_Left) "SphericalTexture" (Variables|Default|GetLeftEyeAtlas))
    (Rendering|Material|SetTextureParameterValue (Variables|Default|GetM_AtlasSphere_Right) "SphericalTexture" (Variables|Default|GetRightEyeAtlas))
    (Development|PrintString "Showing Atlas Sphere ")
    (Rendering|SetVisibility (Variables|Default|GetAtlasSphere_Root) true true)
    (Rendering|SetVisibility (Variables|Default|GetRefLiveCube_Root) false true)))

(fn ConstructionScript
  (bind _returnvalue (Rendering|Material|CreateDynamicMaterialInstance (Variables|Default|GetAtlasSphere_Left) 0 "/StereoPanorama/Assets/MI_AtlasSphereLeft.MI_AtlasSphereLeft" :!class /Script/Engine.PrimitiveComponent))
  (Variables|Default|SetM_AtlasSphere_Left _returnvalue)
  (bind _returnvalue_2 (Rendering|Material|CreateDynamicMaterialInstance (Variables|Default|GetAtlasSphere_Right) 0 "/StereoPanorama/Assets/MI_AtlasSphereRight.MI_AtlasSphereRight" :!class /Script/Engine.PrimitiveComponent))
  (Variables|Default|SetM_AtlasSphere_Right _returnvalue_2))